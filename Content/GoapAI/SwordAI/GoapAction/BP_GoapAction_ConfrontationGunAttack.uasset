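; GOAP action for the sword AI that strafes around the target while performing a walking gun attack.
; On activation it focuses the target, picks a strafe direction opposite to the target's lateral velocity and activates the WalkGunAttack ability by tag.
; Tick applies sideways movement, and the ability re-activates each time it ends until a short random timer expires.
; The action then succeeds, or aborts if the ability is cancelled, clearing focus in both cases.
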(event Custom|EndActionEvent
  ;[1 1 1] Comment
  (Variables|Default|SetTimeIsEnd true))

(event EventReciveonActionActive
  (params (InAIController :type AI%20Controller%20Object%20Reference) (InControlledPawn :type Pawn%20Object%20Reference))
  (bind _returnvalue (Utilities|Name|MakeLiteralName "TargetActor"))
  (bind _blackboard (Variables|/Script/AIModule.AIController|GetBlackboard InAIController))
  (bind _returnvalue_2 (AI|Components|Blackboard|GetValueasObject _blackboard _returnvalue))
  (bind _asactor (Utilities|Casting|CastToActor _returnvalue_2))
  (bind _output_get (Variables|Default|SetIn%20AIController InAIController))
  (AI|SetFocus _output_get _asactor)
  (Variables|Default|SetDirection (Math|Integer|SelectInt -1 1 (> (Math|Vector|DotProduct (Class|KismetMathLibrary|VectorNormal2D (Transformation|GetVelocity _asactor) 0.0001) (Class|KismetMathLibrary|VectorNormal2D (Transformation|GetActorRightVector InControlledPawn) 0.0001)) 0.0)))
  (bind _bresult (Class|GoapActionAbility|ActiveAbilitybyAbilityGroupTag "(TagName=\"SwordAbility.WalkGunAttack\")"))
  (if _bresult
    ;[1 1 1] Comment
    (Utilities|Time|SetTimerbyEvent (delegate Custom|EndActionEvent) (Math|Random|RandomFloatinRange 3.0 4.0))
    (else
      (Class|GoapAction|EndAction "Failed"))))

(event EventReciveonActionTick
  (params (DeltaTime :type Float%20%28single-precision%29) (InAIController :type AI%20Controller%20Object%20Reference) (InControlledPawn :type Pawn%20Object%20Reference))
  (Pawn|Input|AddMovementInput InControlledPawn (* (Transformation|GetActorRightVector InControlledPawn) (Variables|Default|GetDirection)) 0.6 false))

(event EventReciveonAbilityEndDelegate
  (params (GameplayAbilitySpecHandle :type Gameplay%20Ability%20Spec%20Handle%20Structure%20%28by%20ref%29) (bWasCancelled :type Boolean))
  (if bWasCancelled
    (Class|GoapAction|EndAction "Aborted")
    (bind _in_aicontroller (Variables|Default|GetIn%20AIController :!label _label)
      (:then
        (AI|ClearFocus _in_aicontroller))
      (:else))
    (elif (Variables|Default|GetTimeIsEnd)
      (Class|GoapAction|EndAction "Succeeded")
      (goto _label)
      (else
        (Class|GoapActionAbility|ActiveAbilitybyAbilityGroupTag "(TagName=\"SwordAbility.WalkGunAttack\")")))))
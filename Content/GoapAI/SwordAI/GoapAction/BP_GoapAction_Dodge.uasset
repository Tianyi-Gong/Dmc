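; GOAP action for sword AI that performs a dodge through the ability system.
; On activation it triggers the Dodge ability by group tag, focuses the AI controller on the blackboard TargetActor, or fails the action if activation fails.
; When the ability ends, it clears focus and reports failure if the ability was cancelled, success otherwise.
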(event EventReciveonActionActive
  (params (InAIController :type AI%20Controller%20Object%20Reference) (InControlledPawn :type Pawn%20Object%20Reference))
  (Variables|Default|SetIn%20AIController InAIController)
  (bind _bresult (Class|GoapActionAbility|ActiveAbilitybyAbilityGroupTag "(TagName=\"SwordAbility.Avoid.Dodge\")"))
  (if _bresult
    (AI|SetFocus (Variables|Default|GetIn%20AIController) (.AsActor (Utilities|Casting|CastToActor (AI|Components|Blackboard|GetValueasObject (AI|GetBlackboard (Variables|Default|GetIn%20AIController)) (Utilities|Name|MakeLiteralName "TargetActor")))))
    (else
      (Class|GoapAction|EndAction "Failed"))))

(event EventReciveonAbilityEndDelegate
  (params (GameplayAbilitySpecHandle :type Gameplay%20Ability%20Spec%20Handle%20Structure%20%28by%20ref%29) (bWasCancelled :type Boolean))
  (bind _in_aicontroller (Variables|Default|GetIn%20AIController))
  (if bWasCancelled
    (AI|ClearFocus _in_aicontroller)
    (Class|GoapAction|EndAction "Failed")
    (else
      (AI|ClearFocus _in_aicontroller)
      (Class|GoapAction|EndAction "Succeeded"))))
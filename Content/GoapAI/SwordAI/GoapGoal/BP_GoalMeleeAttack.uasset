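; GOAP goal for the sword AI's melee attack, which seeds the agent's private world state when the goal becomes active.
; It reads TargetActor from the AI controller's blackboard and stops if none is valid.
; It sets FaceToTarget from a 2D forward-to-target dot product test and ClosedToTarget from a distance threshold.
; It also resets UseMeleeAttack to false, presumably so the planner must achieve it.
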(event EventReciveonGoalActive
  (params (GoapAgent :type Goap%20Agent%20Component%20Object%20Reference) (InAIController :type AI%20Controller%20Object%20Reference) (InControlledPawn :type Pawn%20Object%20Reference))
  (CallFunction|GoalActive GoapAgent InAIController InControlledPawn))

(fn GoalActive
  (params (GoapAgent :type Goap%20Agent%20Component%20Object%20Reference) (AIController :type AI%20Controller%20Object%20Reference) (ControllPawn :type Pawn%20Object%20Reference))
  (bind _asactor (Utilities|Casting|CastToActor (AI|Components|Blackboard|GetValueasObject (AI|GetBlackboard AIController) (Utilities|Name|MakeLiteralName "TargetActor"))))
  (LocalVariables|SetTargetActor _asactor)
  (Utilities|FlowControl|Sequence
    (:then_0
      ;[1 1 1] FaceToActor
      (Class|GoapAgentComponent|SetGoapPrivateState GoapAgent "(TagName=\"GoapState.FaceToTarget\")" (> (Math|Vector2D|DotProduct(2D) (Math|Conversions|ToVector2D(Vector) (Transformation|GetActorForwardVector ControllPawn)) (Math|Conversions|ToVector2D(Vector) (- (Transformation|GetActorLocation (LocalVariables|GetTargetActor)) (Transformation|GetActorLocation ControllPawn)))) (Class|KismetMathLibrary|DegAcos 5e+01))))
    (:then_1
      ;[1 1 1] ClseToActor
      (Class|GoapAgentComponent|SetGoapPrivateState GoapAgent "(TagName=\"GoapState.ClosedToTarget\")" (< (Math|Vector|Distance(Vector) (Transformation|GetActorLocation (LocalVariables|GetTargetActor)) (Transformation|GetActorLocation ControllPawn)) 2.5e+02)))
    (:then_2
      (Class|GoapAgentComponent|SetGoapPrivateState GoapAgent "(TagName=\"GoapState.UseMeleeAttack\")" false))))
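; AI controller for a GOAP agent that feeds target-related world state into the planner.
; One second after BeginPlay, it stores the first actor tagged "Test1" as blackboard TargetActor and sets HaveTargetActor.
; Before each goal selection, it updates FaceToTarget from an unnormalized 2D dot product against a cosine threshold and ClosedToTarget from a distance check.
; The goal-select delegate clears HaveTargetLocation.
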(event OnGoapGoalSelectDelegate(GoapAgent)
  (params (GoapAgent :type Goap%20Agent%20Component%20Object%20Reference))
  (Class|GoapAgentComponent|SetGoapPrivateState GoapAgent "(TagName=\"GoapState.HaveTargetLocation\")" false))

(event OnPreGoapGoalSelectDelegate(GoapAgent)
  (params (GoapAgent :type Goap%20Agent%20Component%20Object%20Reference))
  (CallFunction|OnPreGoapGoalSelect))

(event Custom|TestLockTarget
  (params (Tag :type Name))
  ;[1 1 1] Comment
  (Utilities|FlowControl|Delay 1.0)
  (bind _outactors (Actor|GetAllActorswithTag Tag))
  (Utilities|IsValid (Utilities|Array|Get(acopy) _outactors)
    (:Is%20Valid
      (AI|Components|Blackboard|SetValueasObject (AI|GetBlackboard 0) (Utilities|Name|MakeLiteralName "TargetActor") (Utilities|Array|Get(acopy) _outactors))
      (Class|GoapAgentComponent|SetGoapPrivateState (Variables|Default|GetGoapAgent) "(TagName=\"GoapState.HaveTargetActor\")" true))))

(event EventBeginPlay
  (CallFunction|TestLockTarget "Test1"))

(event EventTick
  (params (DeltaSeconds :type Float%20%28single-precision%29)))

(fn ConstructionScript)

(fn OnPreGoapGoalSelect
  (bind _returnvalue (Pawn|GetControlledPawn))
  (LocalVariables|SetTargetActor (.AsActor (Utilities|Casting|CastToActor (AI|Components|Blackboard|GetValueasObject (AI|GetBlackboard 0) (Utilities|Name|MakeLiteralName "TargetActor")))))
  (LocalVariables|GetTargetActor
    (:then
      (Utilities|FlowControl|Sequence
        (:then_0
          ;[1 1 1] FaceToActor
          (Class|GoapAgentComponent|SetGoapPrivateState (Variables|Default|GetGoapAgent) "(TagName=\"GoapState.FaceToTarget\")" (> (Math|Vector2D|DotProduct(2D) (Math|Conversions|ToVector2D(Vector) (Transformation|GetActorForwardVector _returnvalue)) (Math|Conversions|ToVector2D(Vector) (- (Transformation|GetActorLocation (LocalVariables|GetTargetActor)) (Transformation|GetActorLocation _returnvalue)))) (Math|Trig|Cos(Degrees) 5e+01))))
        (:then_1
          ;[1 1 1] ClseToActor
          (Class|GoapAgentComponent|SetGoapPrivateState (Variables|Default|GetGoapAgent) "(TagName=\"GoapState.ClosedToTarget\")" (< (Math|Vector|Distance(Vector) (Transformation|GetActorLocation (LocalVariables|GetTargetActor)) (Transformation|GetActorLocation (Pawn|GetControlledPawn))) 2.5e+02)))))
    (:else)))
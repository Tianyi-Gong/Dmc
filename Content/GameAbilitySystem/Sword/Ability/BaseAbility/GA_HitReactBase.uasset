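; Base hit-reaction ability that plays the montage chosen by the character's PoiseManagerComponent on activation and again on each HitReact gameplay event.
; Uppercut impacts also launch the character upward along the hit direction.
; The special air-to-floor loop and end montages then follow their gameplay events.
; A damage immunity effect covers the end montage and is removed when it finishes or the ability ends.
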(event Custom|PlayHitReactMontage
  ;[1 1 1] Comment
  (bind (_result _isspecialanim _outhitmontage _outspecialhitanimconfig) (Class|PoiseManagerComponent|GetLastHitMontageAnim (Variables|Default|GetPoiseManager)))
  (Variables|Default|SetSpecialHitAnimConfig _outspecialhitanimconfig)
  (Utilities|FlowControl|Sequence
    (:then_0
      (|PlayMontageandWaitProxy "None" (select _isspecialanim (.specialhitanimmontagestart (Variables|Default|GetSpecialHitAnimConfig)) _outhitmontage) 1.0 "None" true 1.0 0.0 false
        (:OnCompleted
          (Ability|EndAbility))
        (:OnCancelled
          (Ability|CancelAbility))))
    (:then_1
      (switch Utilities|FlowControl|Switch|SwitchonEActionImpactForce (Variables|/Script/DMCWeaponSystem.PoiseManagerComponent|GetHitActionImpactForce (Variables|Default|GetPoiseManager))
        (:ImpactForce_UpperCut
          (CallFunction|HandUpperCut))))))

(event Custom|HandUpperCut
  ;[1 1 1] Comment
  ;;[1 1 1] Comment
  (Character|LaunchCharacter (Variables|Default|GetAs%20Character) (+ (* (Class|KismetMathLibrary|VectorNormal2D (Variables|/Script/DMCWeaponSystem.PoiseManagerComponent|GetHitWorldDir (Variables|Default|GetPoiseManager)) 0.0001) 1e+02) "0.000000,0.000000,730.000000") true true)
  (Utilities|FlowControl|Sequence
    (:then_0
      (Ability|Tasks|WaitGameplayEvent "(TagName=\"GamePlayEvent.HitAirToFloorLoop\")" 0 true
        (:EventReceived
          (|PlayMontageandWaitProxy "None" (.specialhitanimmontageloop (Variables|Default|GetSpecialHitAnimConfig)) 1.0 "None" true 1.0 0.0 false))))
    (:then_1
      (Ability|Tasks|WaitGameplayEvent "(TagName=\"GamePlayEvent.HitAirToFloorEnd\")" 0 true
        (:then
          (bind _returnvalue (Ability|ApplyGameplayEffectToOwner "/Game/GameAbilitySystem/Sword/Effect/GE_ApplayDamageImmunity.GE_ApplayDamageImmunity_C"))
          (Variables|Default|SetDamageImmunity _returnvalue)
          (|PlayMontageandWaitProxy "None" (.specialhitanimmontageend (Variables|Default|GetSpecialHitAnimConfig)) 1.0 "None" true 1.0 0.0 false
            (:OnCompleted
              (Ability|RemoveGameplayEffectFromOwnerWithHandle (Variables|Default|GetDamageImmunity))
              (Ability|EndAbility))
            (:OnCancelled
              (Ability|RemoveGameplayEffectFromOwnerWithHandle (Variables|Default|GetDamageImmunity))
              (Ability|CancelAbility))))))))

(event Ability|EventActivateAbility
  (bind _returnvalue (Ability|GetAvatarActorfromActorInfo))
  (bind _returnvalue_2 (Actor|GetComponentbyClass _returnvalue "/Script/DMCWeaponSystem.PoiseManagerComponent"))
  (bind _returnvalue_3 (Ability|CommitAbility))
  (if _returnvalue_3
    (Utilities|IsValid _returnvalue_2
      (:Is%20Valid
        (bind _ascharacter (Utilities|Casting|CastToCharacter _returnvalue)
          (:then
            (Variables|Default|SetAs%20Character _ascharacter)
            (Variables|Default|SetPoiseManager _returnvalue_2)
            (Utilities|FlowControl|Sequence
              (:then_0
                (Ability|Tasks|WaitGameplayEvent "(TagName=\"GamePlayEvent.HitReact\")" 0
                  (:EventReceived
                    (CallFunction|PlayHitReactMontage))))
              (:then_1
                (CallFunction|PlayHitReactMontage))))
          (:CastFailed
            (Ability|EndAbility :!label _label))))
      (:Is%20Not%20Valid
        (goto _label)))
    (else
      (goto _label))))

(event Ability|EventOnEndAbility
  (params (bWasCancelled :type Boolean))
  (Ability|RemoveGameplayEffectFromOwnerWithHandle (Variables|Default|GetDamageImmunity)))
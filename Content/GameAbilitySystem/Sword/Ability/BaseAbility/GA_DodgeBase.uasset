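; GA_DodgeBase is a base gameplay ability for a sword dodge.
; On activation it commits the ability and, if the DodgeAnim array has entries, plays a random montage from it through a montage-and-wait task.
; Completion ends the ability and cancellation cancels it, while a failed commit or empty array ends it immediately.
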(event Ability|EventActivateAbility
  (bind _returnvalue (Ability|CommitAbility))
  (if (and _returnvalue (> (Utilities|Array|Length (Variables|Default|GetDodgeAnim)) 0))
    (|PlayMontageandWaitProxy "None" (.OutItem (Utilities|Array|Random (Variables|Default|GetDodgeAnim))) 1.0 "None" true 1.0 0.0 false
      (:OnCompleted
        (Ability|EndAbility))
      (:OnCancelled
        (Ability|CancelAbility)))
    (else
      (Ability|EndAbility))))

(event Ability|EventOnEndAbility
  (params (bWasCancelled :type Boolean)))
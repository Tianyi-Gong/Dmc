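; GA_SwordAttackBase is a Gameplay Ability that runs a montage-based sword combo attack.
; On successful commit it waits for AttackCombo gameplay events and plays the first ComboList montage at reduced rate.
; Each event plays the montage at the current ComboIndex, which increments as each montage starts, until the list runs out.
; Montage completion ends the ability, cancellation cancels it, and a failed commit ends it immediately.
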(event Custom|PlayAttackMontage
  ;[1 1 1] Comment
  (if (<= (Variables|Default|GetComboIndex) (Utilities|Array|LastIndex (Variables|Default|GetComboList)))
    (|PlayMontageandWaitProxy "None" (Utilities|Array|Get(acopy) (Variables|Default|GetComboList) (Variables|Default|GetComboIndex)) 0.75 "None" true 1.0 0.0 false
      (:then
        (Math|Integer|IncrementInt (Variables|Default|GetComboIndex)))
      (:OnCompleted
        (Ability|EndAbility))
      (:OnCancelled
        (Ability|CancelAbility)))))

(event Ability|EventActivateAbility
  (bind _returnvalue (Ability|CommitAbility))
  (if _returnvalue
    (Utilities|FlowControl|Sequence
      (:then_0
        (Ability|Tasks|WaitGameplayEvent "(TagName=\"GamePlayEvent.AttackCombo\")" 0
          (:EventReceived
            (CallFunction|PlayAttackMontage))))
      (:then_1
        (Variables|Default|SetComboIndex 0)
        (CallFunction|PlayAttackMontage)))
    (else
      (Ability|EndAbility))))

(event Ability|EventOnEndAbility
  (params (bWasCancelled :type Boolean)))